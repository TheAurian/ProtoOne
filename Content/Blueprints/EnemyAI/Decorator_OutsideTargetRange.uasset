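; Behavior tree decorator that passes when the enemy's controlled pawn is at or beyond an acceptable distance from its tracked target.
; It casts the owner to EnemyAIController_BP, caches it, and measures the distance between that pawn and the TargetToTrack blackboard actor.
; If the cast fails, it prints an on-screen error and returns false.
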(fn PerformConditionCheck
  (params (OwnerActor :type Actor%20Object%20Reference))
  (bind _asenemy_aicontroller_bp (Utilities|Casting|CastToEnemyAIController_BP OwnerActor)
    (:then
      (Variables|Default|SetAI_CON_Ref _asenemy_aicontroller_bp)
      (return (>= (Math|Vector|VectorLength (- (Transformation|GetActorLocation (AI|BehaviorTree|GetBlackboardValueasActor (Variables|Default|GetTargetToTrack))) (Transformation|GetActorLocation (Pawn|GetControlledPawn (Variables|Default|GetAI_CON_Ref))))) (Variables|Default|GetAcceptableDistance))))
    (:CastFailed
      (Development|PrintString "Unable to Get Enemy AI Controller in Decorator_OutsideTargetRange" true true "(R=0.405000,G=0.015618,B=0.000000,A=1.000000)")
      (return false))))