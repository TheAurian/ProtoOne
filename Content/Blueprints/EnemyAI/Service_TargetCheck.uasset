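; Behavior tree service that lets an enemy detect and track the player character, ProtoOneCharacter_BP.
; Each tick it sphere-traces a wide radius around the controlled pawn, ignoring other enemies, then line-traces on the Camera channel to confirm line of sight.
; A visible player updates the TargetToTrack, TargetLocation and LastKnownLocation blackboard keys.
; A blocked line of sight clears the target and zeroes its location, leaving LastKnownLocation intact.
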(event EventTick
  (params (OwnerActor :type Actor%20Object%20Reference) (DeltaSeconds :type Float%20%28single-precision%29))
  (if (!= (Variables|Default|GetAI_CON_Ref) 0)
    (bind _outactors (Actor|GetAllActorsOfClass "/Game/Blueprints/EnemyAI/EnemyAICharacter_BP.EnemyAICharacter_BP_C" :!label _label))
    (bind _output_get (Variables|Default|SetMyLocation (Transformation|GetActorLocation (Pawn|GetControlledPawn (Variables|Default|GetAI_CON_Ref)))))
    (bind _outhits (Collision|MultiSphereTraceForObjects _output_get (+ (Transformation|GetActorLocation (Pawn|GetControlledPawn (Variables|Default|GetAI_CON_Ref))) "0, 0,15.000000") 1.5e+03 (Variables|Default|GetDesiredObjectTypes) false _outactors "ForDuration"))
    (bind _array_element (Utilities|Array|ForEachLoopwithBreak _outhits :!label _label_2)
      (:LoopBody
        (bind _asproto_one_character_bp (Utilities|Casting|CastToProtoOneCharacter_BP (.HitActor (Collision|BreakHitResult _array_element))))
        (goto _label_2 Break))
      (:Completed
        (bind _outhit (Collision|LineTraceByChannel (Variables|Default|GetMyLocation) (Transformation|GetActorLocation _asproto_one_character_bp) "TraceTypeQuery2" false _outactors "ForDuration"))
        (if (== (.HitActor (Collision|BreakHitResult _outhit)) _asproto_one_character_bp)
          (Class|BTFunctionLibrary|SetBlackboardValueasObject (Variables|Default|GetTargetToTrack) _asproto_one_character_bp)
          (AI|BehaviorTree|SetBlackboardValueasVector (Variables|Default|GetTargetLocation) (Transformation|GetActorLocation _asproto_one_character_bp))
          (AI|BehaviorTree|SetBlackboardValueasVector (Variables|Default|GetLastKnownLocation) (Transformation|GetActorLocation _asproto_one_character_bp))
          (else
            ;[1 1 1] set no targettotrack, and not target location, set lastknownlocation to where the enemy thinks the player was last
            (Class|BTFunctionLibrary|SetBlackboardValueasObject (Variables|Default|GetTargetToTrack))
            (AI|BehaviorTree|SetBlackboardValueasVector (Variables|Default|GetTargetLocation) "0, 0, 0")))))
    (else
      (bind _asenemy_aicontroller_bp (Utilities|Casting|CastToEnemyAIController_BP OwnerActor)
        (:then
          (Variables|Default|SetAI_CON_Ref _asenemy_aicontroller_bp)
          (goto _label))
        (:CastFailed
          (Development|PrintString "Unable to Get Enemy AI Controller in Decorator_OutsideTargetRange" true true "(R=0.405000,G=0.015618,B=0.000000,A=1.000000)"))))))