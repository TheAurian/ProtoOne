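; Behavior tree service that finds and tracks a visible target, intended as the player, for the Tierra AI.
; Each tick it sphere-traces around the controlled pawn for configured object types, ignoring all Tierra characters.
; A Camera-channel line trace checks sight to each hit, writing TargetToFollow and TargetLocation when clear, or clearing only TargetToFollow when blocked.
; The last hit processed decides the target, and nothing updates when the sphere finds nothing.
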(event EventTick
  (params (OwnerActor :type Actor%20Object%20Reference) (DeltaSeconds :type Float%20%28single-precision%29))
  ;[1 1 1] Has AI_CON_Ref been set?
  (if (!= (Variables|Default|GetAI_CON_Ref) 0)
    _
    (else
      ;[1 1 1] Set the ai controller reference
      (bind _astierra_aicontroller_bp (Utilities|Casting|CastToTierraAIController_BP OwnerActor))
      (Variables|Default|SetAI_CON_Ref _astierra_aicontroller_bp)))
  ;[1 1 1] We want to ignore the tierra ai character
  (bind _outactors (Actor|GetAllActorsOfClass "/Game/Blueprints/TierraAI/TierraAICharacter_BP.TierraAICharacter_BP_C"))
  (bind _output_get (Variables|Default|SetMyLocation (Transformation|GetActorLocation (Pawn|GetControlledPawn (Variables|Default|GetAI_CON_Ref)))))
  ;[1 1 1] Get all pawns that are not Tierra
  (bind _outhits (Collision|MultiSphereTraceForObjects _output_get (+ (Transformation|GetActorLocation (Pawn|GetControlledPawn (Variables|Default|GetAI_CON_Ref))) "0, 0,15.000000") 1.5e+03 (Variables|Default|GetDesiredObjectTypes) false _outactors "None"))
  ;[1 1 1] If we get the player pawn
  (bind _array_element (Utilities|Array|ForEachLoopwithBreak _outhits)
    (:LoopBody
      ;[1 1 1] can tierra see the player
      (bind _outhit (Collision|LineTraceByChannel (Variables|Default|GetMyLocation) (Transformation|GetActorLocation (.HitActor (Collision|BreakHitResult _array_element))) "TraceTypeQuery2" false _outactors "None"))
      (if (== (.HitActor (Collision|BreakHitResult _outhit)) (.HitActor (Collision|BreakHitResult _array_element)))
        ;[1 1 1] (true) Set the target and its location to the player
        (Class|BTFunctionLibrary|SetBlackboardValueasObject (Variables|Default|GetTargetToFollow) (.HitActor (Collision|BreakHitResult _outhit)))
        (AI|BehaviorTree|SetBlackboardValueasVector (Variables|Default|GetTargetLocation) (Transformation|GetActorLocation (.HitActor (Collision|BreakHitResult _outhit))))
        (else
          ;[1 1 1] (false) set the target as nothing
          (Class|BTFunctionLibrary|SetBlackboardValueasObject (Variables|Default|GetTargetToFollow)))))))