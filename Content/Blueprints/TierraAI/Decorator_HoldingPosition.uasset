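; Behavior tree decorator for Tierra AI that gates a branch on the pawn's distance from the actor it follows.
; It casts the owner to TierraAIController_BP, stores that reference, and reads TargetToFollow from the blackboard.
; The condition passes when the distance between target and controlled pawn is at least AcceptableDistance, and fails if the cast fails.
; The target is not validity-checked, and NewFunction_0 is an empty stub.
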(fn PerformConditionCheck
  (params (OwnerActor :type Actor%20Object%20Reference))
  (bind _astierra_aicontroller_bp (Utilities|Casting|CastToTierraAIController_BP OwnerActor)
    (:then
      (Variables|Default|SetAI_CON_Ref _astierra_aicontroller_bp)
      (return (>= (Math|Vector|VectorLength (- (Transformation|GetActorLocation (AI|BehaviorTree|GetBlackboardValueasActor (Variables|Default|GetTargetToFollow))) (Transformation|GetActorLocation (Pawn|GetControlledPawn (Variables|Default|GetAI_CON_Ref))))) (Variables|Default|GetAcceptableDistance))))
    (:CastFailed
      (return false))))

(fn NewFunction0
  (params (A :type Object%20Object%20Reference)))